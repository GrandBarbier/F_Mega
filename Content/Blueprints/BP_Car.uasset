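; BP_Car is a physics-driven hover car steered by MoveForward and MoveRight axis input.
; BeginPlay hands CarMesh to four HoverComponents.
; Each Tick traces along the car's down vector; on a hit, distance-scaled force along the surface normal, signed by negated Gravity, replaces world gravity, which returns on a miss.
; Input applies forward force and yaw torque, flipping steering when not moving forward.
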(event `self.ReceiveBeginPlay`
  (`/Game/Blueprints/HoverComponent.InitComponent` (`self.HoverComponent1`) (`self.CarMesh`))
  (`/Game/Blueprints/HoverComponent.InitComponent` (`self.HoverComponent2`) (`self.CarMesh`))
  (`/Game/Blueprints/HoverComponent.InitComponent` (`self.HoverComponent3`) (`self.CarMesh`))
  (`/Game/Blueprints/HoverComponent.InitComponent` (`self.HoverComponent4`) (`self.CarMesh`)))

(event `self.ReceiveTick`
  (params (DeltaSeconds :type "Float (single-precision)"))
  (bind _returnvalue (`SceneComponent.K2_GetComponentLocation` (`self.CarMesh`)))
  (bind (_outhit _returnvalue_2) (`KismetSystemLibrary.LineTraceSingle` :`Start` _returnvalue :`End` (+ _returnvalue (* (`SceneComponent.GetUpVector` (`self.CarMesh`)) (* (`self.TraceLength`) -1.0))) :`TraceChannel` "TraceTypeQuery1" :`DrawDebugType` "ForOneFrame" :`TraceColor` (struct :`R` 0.609675 :`B` 0.75 :`A` 1.0)))
  (if _returnvalue_2
    (bind (_bblockinghit _binitialoverlap _time _distance _location _impactpoint _normal _impactnormal) (`GameplayStatics.BreakHitResult` _outhit))
    (`PrimitiveComponent.AddForce` (`self.CarMesh`) (* _impactnormal (* (`KismetMathLibrary.VSize` (- _location (`SceneComponent.K2_GetComponentLocation` (`self.CarMesh`)))) (* (`self.Gravity`) -1.0))) "None" false)
    (`PrimitiveComponent.SetEnableGravity` (`self.CarMesh`) false)
    (else
      (`PrimitiveComponent.SetEnableGravity` (`self.CarMesh`) true))))

(event `InputAxis|MoveForward`
  (params (AxisValue :type "Float (single-precision)"))
  (`PrimitiveComponent.AddForce` (`self.CarMesh`) (* (* (`SceneComponent.GetForwardVector` (`self.CarMesh`)) (`self.Speed`)) AxisValue) "None" false))

(event `InputAxis|MoveRight`
  (params (AxisValue :type "Float (single-precision)"))
  (bind _returnvalue (`PrimitiveComponent.GetPhysicsLinearVelocity` (`self.CarMesh`) "None"))
  (`PrimitiveComponent.AddTorqueInDegrees` (`self.CarMesh`) (`KismetMathLibrary.MakeVector` 0.0 0.0 (* (`KismetMathLibrary.SelectFloat` 1.0 -1.0 (> (`KismetMathLibrary.Dot_VectorVector` _returnvalue (`SceneComponent.GetForwardVector` (`self.CarMesh`))) 0.0)) (* AxisValue 5000.0))) "None" true))

(fn `UserConstructionScript`)