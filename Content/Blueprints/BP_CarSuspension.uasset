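; Prototype car Blueprint that experiments with raycast suspension on a single physics Body and basic forward movement.
; Each tick a debug-drawn trace runs down the body's up axis; on a hit it disables gravity and applies force along the impact normal, scaled by hit distance and negated Gravity.
; Without a hit, gravity returns.
; The MoveForward axis offsets Body by its forward vector and Speed, without sweep or delta-time scaling.
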(event `self.ReceiveTick`
  (params (DeltaSeconds :type "Float (single-precision)"))
  (bind _returnvalue (`SceneComponent.K2_GetComponentLocation` (`self.Body`)))
  (bind (_outhit _returnvalue_2) (`KismetSystemLibrary.LineTraceSingle` :`Start` _returnvalue :`End` (+ _returnvalue (* (`SceneComponent.GetUpVector` (`self.Body`)) (* (`self.TraceLength`) -1.0))) :`TraceChannel` "TraceTypeQuery1" :`DrawDebugType` "ForOneFrame" :`TraceColor` (struct :`R` 0.609675 :`B` 0.75 :`A` 1.0)))
  (if _returnvalue_2
    (`PrimitiveComponent.SetEnableGravity` (`self.Body`) false)
    (bind (_bblockinghit _binitialoverlap _time _distance _location _impactpoint _normal _impactnormal) (`GameplayStatics.BreakHitResult` _outhit))
    (`PrimitiveComponent.AddForce` (`self.Body`) (* _impactnormal (* (`KismetMathLibrary.VSize` (- _location (`SceneComponent.K2_GetComponentLocation` (`self.Body`)))) (* (`self.Gravity`) -1.0))) "None" false)
    (else
      (`PrimitiveComponent.SetEnableGravity` (`self.Body`) true))))

(event `InputAxis|MoveForward`
  (params (AxisValue :type "Float (single-precision)"))
  (`SceneComponent.K2_AddLocalOffset` (`self.Body`) (* (* (`SceneComponent.GetForwardVector` (`self.Body`)) (`self.Speed`)) AxisValue) false false))

(fn `UserConstructionScript`)